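; Falling platform that drops after BP_Bob overlaps its trigger, then returns to its starting spot and rearms.
; Activation saves the platform transform, waits briefly, then enables physics simulation for a timed fall.
; Reset disables physics and uses a timeline to lerp the transform back to the start.
; An Activated flag blocks retriggering mid-cycle, while material swaps, sounds and debug text mark each stage.
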(event `self.ReceiveBeginPlay`)

(event `self.Trigger.OnComponentBeginOverlap`
  (params (OverlappedComponent :type "PrimitiveComponent Object Reference") (OtherActor :type "Actor Object Reference") (OtherComp :type "PrimitiveComponent Object Reference") (OtherBodyIndex :type Integer) (bFromSweep :type Boolean) (SweepResult :type "HitResult Structure (by ref)"))
  (cast `/Game/Coding1/Blueprints/BP_Bob` OtherActor)
  (`self.ActivateFallingPlatform`))

(event `ActivateFallingPlatform`
  (if (not (`self.Activated`))
    (set `self.Activated` true)
    (`GameplayStatics.PlaySoundAtLocation` "/Game/Coding1/Audio/boom.boom" (`self.K2_GetActorLocation`) (struct) 1.0 (`KismetMathLibrary.RandomFloatInRange` 9.5 1.05) 0.0 "/Game/Coding1/Audio/NewSoundAttenuation.NewSoundAttenuation" null null null)
    (`PrimitiveComponent.SetMaterial` (`self.Platform`) 0 "/Engine/MapTemplates/Materials/BasicAsset03.BasicAsset03")
    (set `self.Start` (`SceneComponent.K2_GetComponentToWorld` (`self.Platform`)))
    (`KismetSystemLibrary.PrintText` "We will stay in the air for 1 second.")
    (`KismetSystemLibrary.Delay` 1.0)
    (`self.StartFalling`)))

(event `StartFalling`
  (`KismetSystemLibrary.PrintText` "We're gonna fall for 5 seconds.")
  (`PrimitiveComponent.SetMaterial` (`self.Platform`) 0 "/Landmass/Landscape/BlueprintBrushes/Materials/Debug/M_Sphere.M_Sphere")
  (`PrimitiveComponent.SetSimulatePhysics` (`self.Platform`) true)
  (`KismetSystemLibrary.Delay` 5.0)
  (`self.ResetPlatform`))

(event `ResetPlatform`
  (`KismetSystemLibrary.PrintText` "Returning to start...")
  (`PrimitiveComponent.SetMaterial` (`self.Platform`) 0 "/Engine/ArtTools/RenderToTexture/Materials/Debug/M_TestFlipbookAnimation.M_TestFlipbookAnimation")
  (`PrimitiveComponent.SetSimulatePhysics` (`self.Platform`) false)
  (set `self.End` (`SceneComponent.K2_GetComponentToWorld` (`self.Platform`)))
  (bind (_direction _newtrack_0) (`Timeline|ReturnToStart` :!via `PlayFromStart`)
    (:`Update`
      (`SceneComponent.K2_SetWorldTransform` (`self.Platform`) (`KismetMathLibrary.TLerp` (`self.End`) (`self.Start`) _newtrack_0) false false))
    (:`Finished`
      (`KismetSystemLibrary.PrintText` "Platform is Reset.")
      (set `self.Activated` false) ; platform ready to be activated again
      (`PrimitiveComponent.SetMaterial` (`self.Platform`) 0 "/Engine/BufferVisualization/BaseColor.BaseColor")
      (`GameplayStatics.PlaySoundAtLocation` "/Game/Coding1/Audio/boom.boom" (`self.K2_GetActorLocation`) (struct) 1.0 1.1 0.0 "/Game/Coding1/Audio/NewSoundAttenuation.NewSoundAttenuation" null null null))))

(fn `UserConstructionScript`)